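; BP_GridTile is a minigame grid tile that changes material with its hazard state: safe ice, spawn warning, deadly orca (Syachi) or vanishing orca.
; OnTileStateChanged builds dynamic material instances for the three non-safe states, writing MoveInterval to SyachiRotation in both blink states.
; The vanishing state creates its instance without applying it to TileMesh.
; The Direction-to-rotation mapping and a final SetMaterial are unconnected, so Direction has no effect.
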(event EventOnTileStateChanged
  (params (NewState :type ETileState%20Enum :default "Safe") (MoveInterval :type Float%20%28single-precision%29) (Direction :type EGridDirection8%20Enum :default "None"))
  (switch Utilities|FlowControl|Switch|SwitchonETileState NewState
    (:Safe
      (Rendering|Material|SetMaterial (Variables|Default|GetTileMesh) 0 "/Game/MiniGame/images/M_Ice.M_Ice"))
    (:Warning
      (Rendering|Material|SetScalarParameterValue 0 (Variables|Default|GetSyachiRotation) MoveInterval :!class /Script/Engine.KismetMaterialLibrary)
      (bind _returnvalue (Rendering|Material|CreateDynamicMaterialInstance (Variables|Default|GetTileMesh) 0 "/Game/MiniGame/images/M_BlinkYellow.M_BlinkYellow" "None" :!class /Script/Engine.PrimitiveComponent))
      (bind _output_get (Variables|Default|SetTileMID _returnvalue))
      (Rendering|Material|SetMaterial (Variables|Default|GetTileMesh) 0 _output_get))
    (:ActiveHazard
      (bind _returnvalue_2 (Rendering|Material|CreateDynamicMaterialInstance (Variables|Default|GetTileMesh) 0 "/Game/MiniGame/images/M_Syachi.M_Syachi" "None" :!class /Script/Engine.PrimitiveComponent))
      (bind _output_get_2 (Variables|Default|SetTileMID _returnvalue_2))
      (Rendering|Material|SetMaterial (Variables|Default|GetTileMesh) 0 _output_get_2))
    (:ExpiringHazard
      (Rendering|Material|SetScalarParameterValue 0 (Variables|Default|GetSyachiRotation) MoveInterval :!class /Script/Engine.KismetMaterialLibrary)
      (bind _returnvalue_3 (Rendering|Material|CreateDynamicMaterialInstance (Variables|Default|GetTileMesh) 0 "/Game/MiniGame/images/M_BlinkSyachi.M_BlinkSyachi" "None" :!class /Script/Engine.PrimitiveComponent))
      (bind _output_get_3 (Variables|Default|SetTileMID _returnvalue_3)))))

(fn ConstructionScript)